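; Aeon component that streams level instances on a transformable 2D or 3D grid around a target actor.
; Each tick it probes coordinates near the Loader volume with a reference cell, spawning tagged trigger boxes where they overlap.
; Configurable Loader and Unloader overlap events load or hide and unload each cell's level instance, chosen by LevelPicker.
; In 2D mode, per-column counts keep a level loaded until its last vertical cell unloads.
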(event Custom|Event%20OnLoadCell
  (params (OverlappedActor :type Actor%20Object%20Reference) (OtherActor :type Actor%20Object%20Reference))
  (Internal|LoadCell OtherActor))

(event Custom|Event%20OnUnloadCell
  (params (OverlappedActor :type Actor%20Object%20Reference) (OtherActor :type Actor%20Object%20Reference))
  (Internal|UnloadCell OtherActor))

(event Custom|Event%20Deactivated
  ;[0 0 0] Unregister Loader
  (switch Utilities|FlowControl|Switch|SwitchonE_Aeon_TriggerEvent (Variables|Loader|GetLoaderTrigger)
    (:NewEnumerator0
      (Collision|UnbindEventfromOnActorBeginOverlap (Variables|Internal|GetLoader) (delegate Custom|Event%20OnLoadCell)))
    (:NewEnumerator1
      (EventDispatchers|UnbindEventfromOnActorEndOverlap (Variables|Internal|GetLoader) (delegate Custom|Event%20OnLoadCell))))
  ;[0 0 0] Unregister Unloader
  (switch Utilities|FlowControl|Switch|SwitchonE_Aeon_TriggerEvent (Variables|Unloader|GetUnloaderTrigger)
    (:NewEnumerator0
      (Collision|UnbindEventfromOnActorBeginOverlap (Variables|Internal|GetUnloader) (delegate Custom|Event%20OnUnloadCell)))
    (:NewEnumerator1
      (EventDispatchers|UnbindEventfromOnActorEndOverlap (Variables|Internal|GetUnloader) (delegate Custom|Event%20OnUnloadCell)))))

(event Custom|Event%20Activated
  ;[0 0 0] Register Loader
  (switch Utilities|FlowControl|Switch|SwitchonE_Aeon_TriggerEvent (Variables|Loader|GetLoaderTrigger)
    (:NewEnumerator0
      (EventDispatchers|AssignOnActorBeginOverlap (Variables|Internal|GetLoader) (delegate Custom|Event%20OnLoadCell)))
    (:NewEnumerator1
      (EventDispatchers|AssignOnActorEndOverlap (Variables|Internal|GetLoader) (delegate Custom|Event%20OnLoadCell))))
  ;[0 0 0] Register Unloader
  (switch Utilities|FlowControl|Switch|SwitchonE_Aeon_TriggerEvent (Variables|Unloader|GetUnloaderTrigger)
    (:NewEnumerator0
      (EventDispatchers|AssignOnActorBeginOverlap (Variables|Internal|GetUnloader) (delegate Custom|Event%20OnUnloadCell)))
    (:NewEnumerator1
      (EventDispatchers|AssignOnActorEndOverlap (Variables|Internal|GetUnloader) (delegate Custom|Event%20OnUnloadCell)))))

(event EventBeginPlay
  ;[0 0 0] Check if Auto Activated
  (if (Variables|Activation|GetbAutoActivate)
    ;[0 0 0] Activate
    (Public|ActivateComp)))

(event EventTick
  (params (DeltaSeconds :type Float%20%28single-precision%29))
  ;[0 0 0] If Activated
  (if (Variables|Internal|GetbIsActivated)
    (Internal|OnTick)))

(fn ActivateComp
  ;[0 0 0] If Not Activated
  (if (not (Variables|Internal|GetbIsActivated))
    ;[0 0 0] Initialize
    (bind _initialized (Internal|Init))
    (if _initialized
      ;[0 0 0] Mark Activated
      (Variables|Internal|SetbIsActivated true)
      (Components|Tick|SetComponentTickEnabled true)
      (CallFunction|EventActivated)
      (return true)
      (else
        (return false)))))

(fn Clear
  (Utilities|FlowControl|Sequence
    (:then_0
      ;[0 0 0] Clear Cell
      (Utilities|IsValid (Variables|Internal|GetCell)
        (:Is%20Valid
          (Actor|DestroyActor (Variables|Internal|GetCell))
          (Variables|Internal|SetCell 0))))
    (:then_1
      ;[0 0 0] Clear Cells
      (bind _values (Utilities|Map|Values (Variables|Internal|GetCells)))
      (for _array_element _values
        (Actor|DestroyActor _array_element))
      (Utilities|Map|Clear (Variables|Internal|GetCells)))
    (:then_2
      ;[0 0 0] Clear Cells Loaded
      (Utilities|Set|Clear (Variables|Internal|GetCellsLoaded)))
    (:then_3
      ;[0 0 0] Clear Grid
      (Utilities|IsValid (Variables|Internal|GetGrid)
        (:Is%20Valid
          (Actor|DestroyActor (Variables|Internal|GetGrid))
          (Variables|Internal|SetGrid 0))))
    (:then_4
      ;[0 0 0] Clear Level Picker
      (Default|Clear (Variables|LevelPicker|GetLevelPicker)))
    (:then_5
      ;[0 0 0] Clear Levels
      (bind _values_2 (Utilities|Map|Values (Variables|Internal|GetLevels)))
      (for _array_element_2 _values_2
        (Class|LevelStreaming|SetIsRequestingUnloadandRemoval _array_element_2 true))
      (Utilities|Map|Clear (Variables|Internal|GetLevels)))
    (:then_6
      ;[0 0 0] Clear Loader
      (Utilities|IsValid (Variables|Internal|GetLoader)
        (:Is%20Valid
          (Actor|DestroyActor (Variables|Internal|GetLoader))
          (Variables|Internal|SetLoader 0))))
    (:then_7
      ;[0 0 0] Clear Verts
      (Utilities|Map|Clear (Variables|Internal|GetVerts)))
    (:then_8
      ;[0 0 0] Clear Unloader
      (Utilities|IsValid (Variables|Internal|GetUnloader)
        (:Is%20Valid
          (Actor|DestroyActor (Variables|Internal|GetUnloader))
          (Variables|Internal|SetUnloader 0))))))

(fn CreateCell
  (Utilities|FlowControl|Sequence
    (:then_0
      ;[0 0 0] Create Actor
      (bind _returnvalue (Game|SpawnActorfromClass "/Script/Engine.TriggerBox" (Math|Transform|MakeTransform "-2147483648.000000,-2147483648.000000,-2147483648.000000" "0, 0, 0" "1.000000,1.000000,1.000000") "AlwaysSpawn" "MultiplyWithRoot" 0 0))
      (LocalVariables|SetCurCell _returnvalue))
    (:then_1
      ;[0 0 0] Set Visibility
      (Rendering|SetActorHiddenInGame (LocalVariables|GetCurCell) (Math|Boolean|NANDBoolean (Variables|Debug|GetbDebug) (Variables|Debug|GetbShowCells))))
    (:then_2
      ;[0 0 0] Set Scale
      (Transformation|SetActorScale3D (LocalVariables|GetCurCell) (Utilities|Operators|Divide (Variables|Grid|GetCellSize) (.BoxExtent (Collision|GetComponentBounds (Variables|/Script/Engine.TriggerBase|GetCollisionComponent (LocalVariables|GetCurCell)))) 2.0)))
    (:then_3
      ;[0 0 0] Add to Grid
      (Transformation|AttachActorToActor (LocalVariables|GetCurCell) (Variables|Internal|GetGrid) "None" "KeepRelative" "KeepRelative" "KeepRelative" false)
      (Actor|SetOwner (LocalVariables|GetCurCell) (Variables|Internal|GetGrid)))
    (:then_4
      ;[0 0 0] Add Grid Tag
      (Variables|/Script/Engine.Actor|SetTags (LocalVariables|GetCurCell) (Utilities|Array|MakeArray (Variables|Internal|GetGridTag))))
    (:then_5
      (return (LocalVariables|GetCurCell)))))

(fn CreateLevel
  (params (Coord :type Int%20Vector%20Structure))
  ;[0 0 0] Pick Level
  (bind _levelname (Default|GetLevelName (Variables|LevelPicker|GetLevelPicker) Coord))
  ;[0 0 0] Create Level
  (bind _returnvalue (Class|LevelStreaming|CreateInstance (Class|GameplayStatics|GetStreamingLevel _levelname) (Utilities|String|Append (Utilities|String|ToString(Integer) (.x Coord)) "_" (Utilities|String|ToString(Integer) (.y Coord)) "_" (Utilities|String|ToString(Integer) (.z Coord)) "_" (LocalVariables|GetName))))
  (return _returnvalue))

(fn CreateStaticMeshActor
  (params (Mesh :type Static%20Mesh%20Object%20Reference) (Transform :type Transform) (Visible :type Boolean) (Material :type Material%20Instance%20Object%20Reference))
  (Utilities|FlowControl|Sequence
    (:then_0
      ;[0 0 0] Create Actor
      (bind _returnvalue (Game|SpawnActorfromClass "/Script/Engine.StaticMeshActor" Transform "AlwaysSpawn" "MultiplyWithRoot" 0 0))
      (LocalVariables|SetcurActor _returnvalue))
    (:then_1
      ;[0 0 0] Set Visibility
      (Rendering|SetActorHiddenInGame (LocalVariables|GetcurActor) (Math|Boolean|NANDBoolean (Variables|Debug|GetbDebug) Visible)))
    (:then_2
      ;[0 0 0] Create Static Mesh
      (LocalVariables|SetmeshComp (Variables|/Script/Engine.StaticMeshActor|GetStaticMeshComponent (LocalVariables|GetcurActor)))
      (Transformation|SetMobility (LocalVariables|GetmeshComp) "Movable")
      (Components|StaticMesh|SetStaticMesh (LocalVariables|GetmeshComp) Mesh)
      (Rendering|Material|SetMaterial (LocalVariables|GetmeshComp) 0 Material))
    (:then_3
      ;[0 0 0] Configure Collision
      (Collision|SetCollisionObjectType (LocalVariables|GetmeshComp) "ECC_WorldDynamic")
      (Collision|SetCollisionResponsetoAllChannels (LocalVariables|GetmeshComp) "ECR_Overlap")
      (Collision|SetCollisionEnabled (LocalVariables|GetmeshComp) "QueryOnly")
      (Variables|/Script/Engine.PrimitiveComponent|SetbGenerateOverlapEvents (LocalVariables|GetmeshComp) true))
    (:then_4
      ;[0 0 0] Other
      (Rendering|SetCastShadow (LocalVariables|GetmeshComp) false))
    (:then_5
      (return (LocalVariables|GetcurActor)))))

(fn CreateTag
  (return (Utilities|String|StringToName (Utilities|String|Append (Utilities|String|ToString(Text) (Utilities|Text|MakeLiteralText "Name")) "_" (Utilities|String|ToString(Integer) (Class|KismetMathLibrary|RandomIntegerfromStream (Variables|Internal|GetRandomStream) 1000000000))))))

(fn DeactivateComp
  ;[0 0 0] If Activated
  (if (Variables|Internal|GetbIsActivated)
    ;[0 0 0] Mark Deactivated
    (Variables|Internal|SetbIsActivated false)
    ;[0 0 0] Trigger Deactivated Event
    (CallFunction|EventDeactivated)))

(fn GetorCreateLevel
  (params (Coord :type Int%20Vector%20Structure))
  (bind _grid (Variables|Internal|GetGrid))
  (bind _levels (Variables|Internal|GetLevels))
  (bind _returnvalue (Transformation|GetActorTransform _grid))
  (bind (_value _returnvalue_2) (Utilities|Map|Find _levels Coord))
  (Utilities|FlowControl|Sequence
    (:then_0
      ;[0 0 0] Check if Level Exists
      (if _returnvalue_2
        (LocalVariables|SetLevel _value)
        (else
          ;[0 0 0] Create level
          (bind _level (Internal|CreateLevel Coord))
          (bind _output_get (LocalVariables|SetLevel _level))
          (Variables|/Script/Engine.LevelStreaming|SetLevelTransform _output_get (Math|Transform|MakeTransform (Public|GridtoWorld (Public|FromCoord Coord)) (.rotation _returnvalue) (.scale _returnvalue)))
          ;[0 0 0] Save Level
          (Utilities|Map|Add (Variables|Internal|GetLevels) Coord (LocalVariables|GetLevel)))))
    (:then_1
      (return (LocalVariables|GetLevel)))))

(fn Init
  (Utilities|FlowControl|Sequence
    (:then_0
      ;[0 0 0] Init Target
      (bind _success (Internal|InitTarget))
      (if (not _success)
        (return false)))
    (:then_1
      ;[0 0 0] Configure Random Stream
      ;;[0 0 0] Check if Using Random Seed
      (if (Variables|Config|GetbRandomSeed)
        ;;[0 0 0] Get Random Seed
        (Class|KismetMathLibrary|SeedRandomStream (Variables|Internal|GetRandomStream))
        (else
          ;;[0 0 0] Make Random Stream
          (bind _output_get (Variables|Internal|SetRandomStream ""))
          (Math|Random|SetRandomStreamSeed _output_get (Variables|Config|GetSeed)))))
    (:then_2
      ;[0 0 0] Check Level Picker Instance
      (Utilities|IsValid (Variables|LevelPicker|GetLevelPicker)
        (:Is%20Valid
          _)
        (:Is%20Not%20Valid
          ;[0 0 0] Create Level Picker Instance from Class
          (bind _returnvalue (Game|ConstructObjectfromClass (Variables|LevelPicker|GetLevelPickerClass) (Variables|Internal|GetRandomStream)))
          (bind _output_get_2 (Variables|LevelPicker|SetLevelPicker _returnvalue))))
      ;[0 0 0] Initialize Level Picker
      (bind _success_2 (Default|Init _output_get_2))
      (if (not _success_2)
        (return false)))
    (:then_3
      ;[0 0 0] Get Loader
      ;;[0 0 0] Check if Actor Provided
      (Utilities|IsValid (Variables|Internal|GetLoader)
        (:Is%20Not%20Valid
          ;;[0 0 0] Check if Mesh Provided
          (Utilities|IsValid (Variables|Loader|GetLoaderMesh)
            (:Is%20Valid
              ;;[0 0 0] Create Render Actor
              (bind _actor (Internal|CreateStaticMeshActor (Variables|Loader|GetLoaderMesh) (Variables|Loader|GetLoaderTransform) (Variables|Debug|GetbShowLoader) (Variables|Loader|GetLoaderMaterial)))
              (Variables|Internal|SetLoader _actor))
            (:Is%20Not%20Valid
              ;;[0 0 0] Log Warning
              (Internal|Log (Utilities|String|ToString(Text) (Utilities|Text|MakeLiteralText "Error_MissingLoaderMesh")))
              (return false))))))
    (:then_4
      ;[0 0 0] Get Unloader
      ;;[0 0 0] Check if Actor Provided
      (Utilities|IsValid (Variables|Internal|GetUnloader)
        (:Is%20Not%20Valid
          ;;[0 0 0] Check if Mesh Provided
          (Utilities|IsValid (Variables|Unloader|GetUnloaderMesh)
            (:Is%20Valid
              ;;[0 0 0] Create Render Actor
              (bind _actor_2 (Internal|CreateStaticMeshActor (Variables|Unloader|GetUnloaderMesh) (Variables|Unloader|GetUnloaderTransform) (Variables|Debug|GetbShowUnloader) (Variables|Unloader|GetUnloaderMaterial)))
              (Variables|Internal|SetUnloader _actor_2))
            (:Is%20Not%20Valid
              ;;[0 0 0] Log Warning
              (Internal|Log (Utilities|String|ToString(Text) (Utilities|Text|MakeLiteralText "Error_MissingUnloaderMesh")))
              (return false))))))
    (:then_5
      ;[0 0 0] Attach Loader to Target
      (Transformation|AttachActorToActor (Variables|Internal|GetLoader) (Variables|Config|GetTarget) "None" "KeepRelative" "KeepRelative" "KeepRelative" false)
      ;[0 0 0] Attach Unloader to Target
      (Transformation|AttachActorToActor (Variables|Internal|GetUnloader) (Variables|Config|GetTarget) "None" "KeepRelative" "KeepRelative" "KeepRelative" false))
    (:then_6
      ;[0 0 0] Create Grid
      ;;[0 0 0] Generate Grid Tag
      (Variables|Internal|SetGridTag (Internal|CreateTag))
      ;;[0 0 0] Create Grid Actor
      (bind _returnvalue_2 (Game|SpawnActorfromClass "/Script/Engine.Actor" (Math|Transform|MakeTransform "0, 0, 0" "0, 0, 0" "1.000000,1.000000,1.000000") "AlwaysSpawn" "MultiplyWithRoot" 0 0))
      (bind _output_get_3 (Variables|Internal|SetGrid _returnvalue_2))
      (Game|AddComponentbyClass _output_get_3 "/Script/Engine.SceneComponent" false (Variables|Grid|GetGridTransform)))
    (:then_7
      ;[0 0 0] Create Reference Cell
      (bind _cell (Internal|CreateCell))
      (bind _output_get_4 (Variables|Internal|SetCell _cell))
      (Variables|/Script/Engine.Actor|SetTags _output_get_4 (Utilities|Array|MakeArray))
      (Rendering|SetActorHiddenInGame (Variables|Internal|GetCell) true))
    (:then_8
      (return true))))

(fn InitTarget
  ;[0 0 0] Check if Actor Given
  (Utilities|IsValid (Variables|Config|GetTarget)
    (:Is%20Valid
      (return true))
    (:Is%20Not%20Valid
      ;[0 0 0] Check if Owner is a Player Controller
      (bind _asplayer_controller (Utilities|Casting|CastToPlayerController (Components|GetOwner))
        (:then
          ;[0 0 0] Use Controller Pawn
          (bind _output_get (Variables|Config|SetTarget (Pawn|GetControlledPawn _asplayer_controller)))
          ;[0 0 0] Check if Valid
          (Utilities|IsValid _output_get
            (:Is%20Valid
              _)
            (:Is%20Not%20Valid
              ;[0 0 0] Log Warning
              (Internal|Log (Utilities|String|ToString(Text) (Utilities|Text|MakeLiteralText "Error_MissingTarget")) :!label _label)
              (return false))))
        (:CastFailed
          ;[0 0 0] Use Owner
          (bind _output_get_2 (Variables|Config|SetTarget (Components|GetOwner)))
          (Utilities|IsValid _output_get_2
            (:Is%20Valid
              _)
            (:Is%20Not%20Valid
              (goto _label)))))
      (return true))))

(fn LoadCell
  (params (Cell :type Actor%20Object%20Reference))
  ;[0 0 0] Check if Grid Cell
  (if (Actor|ActorHasTag Cell (Variables|Internal|GetGridTag))
    (Utilities|FlowControl|Sequence
      (:then_0
        ;[0 0 0] Get Coord
        (LocalVariables|SetCoord (Utilities|Round(Vector) (Public|ToCoord (Public|WorldtoGrid (Transformation|GetActorLocation Cell))))))
      (:then_1
        ;[0 0 0] Check if Loaded
        (if (Utilities|Set|Contains (Variables|Internal|GetCellsLoaded) (LocalVariables|GetCoord))
          (return)))
      (:then_2
        ;[0 0 0] Adjust for Verticality
        (if (Variables|Grid|GetbIs3D%20Grid)
          (LocalVariables|SetLevelCoord (LocalVariables|GetCoord))
          (else
            (LocalVariables|SetLevelCoord (Utilities|Struct|MakeIntVector (.x (LocalVariables|GetCoord)) (.y (LocalVariables|GetCoord)) 0)))))
      (:then_3
        ;[0 0 0] Get Or Create Level
        (bind _levelstream (Internal|GetorCreateLevel (LocalVariables|GetLevelCoord)))
        (LocalVariables|SetLevel _levelstream))
      (:then_4
        ;[0 0 0] Load Level
        (Variables|/Script/Engine.LevelStreaming|SetbShouldBeLoaded (LocalVariables|GetLevel) true)
        (Variables|/Script/Engine.LevelStreaming|SetbShouldBeVisible (LocalVariables|GetLevel) true))
      (:then_5
        ;[0 0 0] Update Vert Count
        (Utilities|Map|Add (Variables|Internal|GetVerts) (Utilities|Struct|MakeIntVector (.x (LocalVariables|GetCoord)) (.y (LocalVariables|GetCoord)) 0) (+ (.Value (Utilities|Map|Find (Variables|Internal|GetVerts) (Utilities|Struct|MakeIntVector (.x (LocalVariables|GetCoord)) (.y (LocalVariables|GetCoord)) 0))) 1)))
      (:then_6
        ;[0 0 0] Save Loaded Cell
        (Utilities|Set|Add (Variables|Internal|GetCellsLoaded) (LocalVariables|GetCoord))))))

(fn Log
  (params (Message :type String))
  (Development|PrintString (Utilities|String|Append "[" (Utilities|String|ToString(Text) (Utilities|Text|MakeLiteralText "Name")) "] " Message) (Variables|Debug|GetbDebug) true "(R=0.000000,G=0.660000,B=1.000000,A=1.000000)" 1e+01))

(fn OnTick
  (bind _loader (Variables|Internal|GetLoader))
  (bind (_origin _boxextent) (Collision|GetActorBounds _loader false false))
  (bind _returnvalue (* _boxextent 2.0))
  (bind _returnvalue_2 (+ _origin _returnvalue))
  (bind _returnvalue_3 (- _origin _returnvalue))
  (bind _output (Public|WorldtoGrid _returnvalue_2))
  (bind _output_2 (Public|WorldtoGrid _returnvalue_3))
  (Utilities|FlowControl|Sequence
    (:then_0
      ;[0 0 0] Get Loader Volume in Cell Units
      (LocalVariables|SetExtentMin (Utilities|Floor(Vector) (Public|ToCoord (Utilities|Min(Vectors) _output_2 _output))))
      (LocalVariables|SetExtentMax (Utilities|Ceil(Vector) (Public|ToCoord (Utilities|Max(Vectors) _output_2 _output)))))
    (:then_1
      ;[0 0 0] Get List of Coords within Volume
      ;;[0 0 0] For Each X Coord
      (for _index (range (.x (LocalVariables|GetExtentMin)) (.x (LocalVariables|GetExtentMax)))
        (LocalVariables|SetcurX _index)
        ;;[0 0 0] For Each Y Coord
        (for _index_2 (range (.y (LocalVariables|GetExtentMin)) (.y (LocalVariables|GetExtentMax)))
          (LocalVariables|SetcurY _index_2)
          ;;[0 0 0] For Each Z Coord
          (for _index_3 (range (.z (LocalVariables|GetExtentMin)) (.z (LocalVariables|GetExtentMax)))
            (LocalVariables|SetcurZ _index_3)
            ;;[0 0 0] Save Coord
            (Utilities|Array|Add (LocalVariables|GetCoords) (Utilities|Struct|MakeIntVector (LocalVariables|GetcurX) (LocalVariables|GetcurY) (LocalVariables|GetcurZ)))))))
    (:then_2
      ;[0 0 0] Create Overlapping Cells
      ;;[0 0 0] For Each Coord
      (for _array_element (LocalVariables|GetCoords)
        (LocalVariables|SetcurCoord _array_element)
        ;;[0 0 0] Check if Already Exists
        (if (not (Utilities|Map|Contains (Variables|Internal|GetCells) (LocalVariables|GetcurCoord)))
          ;;[0 0 0] Move Ref Cell
          (Transformation|SetActorRelativeLocation (Variables|Internal|GetCell) (Public|FromCoord (LocalVariables|GetcurCoord)))
          ;;[0 0 0] Check for Overlap
          (if (Collision|IsOverlappingActor (Variables|Internal|GetLoader) (Variables|Internal|GetCell) :!class /Script/Engine.Actor)
            ;;[0 0 0] Create Actual Cell
            (bind _cell (Internal|CreateCell))
            (LocalVariables|SetcurCell _cell)
            ;;[0 0 0] Save Cell Ref
            (Utilities|Map|Add (Variables|Internal|GetCells) (LocalVariables|GetcurCoord) (LocalVariables|GetcurCell))
            ;;[0 0 0] Move to Location
            (Transformation|SetActorRelativeLocation (LocalVariables|GetcurCell) (Public|FromCoord (LocalVariables|GetcurCoord)))))))))

(fn UnloadCell
  (params (Cell :type Actor%20Object%20Reference))
  ;[0 0 0] Check if Grid Cell
  (if (Actor|ActorHasTag Cell (Variables|Internal|GetGridTag))
    (Utilities|FlowControl|Sequence
      (:then_0
        ;[0 0 0] Get Coord
        (LocalVariables|SetCoord (Utilities|Round(Vector) (Public|ToCoord (Public|WorldtoGrid (Transformation|GetActorLocation Cell))))))
      (:then_1
        ;[0 0 0] Check if Loaded
        (if (not (Utilities|Set|Contains (Variables|Internal|GetCellsLoaded) (LocalVariables|GetCoord)))
          (return)))
      (:then_2
        ;[0 0 0] Adjust for Verticality
        (if (Variables|Grid|GetbIs3D%20Grid)
          (LocalVariables|SetLevelCoord (LocalVariables|GetCoord))
          (else
            (LocalVariables|SetLevelCoord (Utilities|Struct|MakeIntVector (.x (LocalVariables|GetCoord)) (.y (LocalVariables|GetCoord)) 0)))))
      (:then_3
        ;[0 0 0] Update Vert Count
        (LocalVariables|SetvertCount (- (.Value (Utilities|Map|Find (Variables|Internal|GetVerts) (Utilities|Struct|MakeIntVector (.x (LocalVariables|GetCoord)) (.y (LocalVariables|GetCoord)) 0))) 1))
        (Utilities|Map|Add (Variables|Internal|GetVerts) (Utilities|Struct|MakeIntVector (.x (LocalVariables|GetCoord)) (.y (LocalVariables|GetCoord)) 0) (LocalVariables|GetvertCount)))
      (:then_4
        ;[0 0 0] Remove Cell
        (Actor|DestroyActor Cell)
        (Utilities|Map|Remove (Variables|Internal|GetCells) (LocalVariables|GetCoord))
        (Utilities|Set|Remove (Variables|Internal|GetCellsLoaded) (LocalVariables|GetCoord)))
      (:then_5
        ;[0 0 0] Check if Loading Vertically
        (if (not (Variables|Grid|GetbIs3D%20Grid))
          ;[0 0 0] If Not Vertical, Check Vert Count
          (if (not (<= (LocalVariables|GetvertCount) 0))
            (return))))
      (:then_6
        ;[0 0 0] Check if Level Exists
        (if (.ReturnValue (Utilities|Map|Find (Variables|Internal|GetLevels) (LocalVariables|GetLevelCoord)))
          (LocalVariables|SetLevel (.Value (Utilities|Map|Find (Variables|Internal|GetLevels) (LocalVariables|GetLevelCoord))))
          (else
            (return))))
      (:then_7
        ;[0 0 0] Unload Level
        (Variables|/Script/Engine.LevelStreaming|SetbShouldBeLoaded (LocalVariables|GetLevel) false)
        (Variables|/Script/Engine.LevelStreaming|SetbShouldBeVisible (LocalVariables|GetLevel) false)))))

(fn FromCoord
  (params (Coord :type Int%20Vector%20Structure))
  (return (* (Math|Conversions|ToVector(Float) Coord) (Variables|Grid|GetCellSize))))

(fn GridtoWorld
  (params (Input :type Vector))
  (bind _grid (Variables|Internal|GetGrid))
  (bind _returnvalue (Transformation|GetActorTransform _grid))
  (return (+ (.location _returnvalue) (Math|Vector|RotateVector (* (.scale _returnvalue) Input) (.rotation _returnvalue)))))

(fn ToCoord
  (params (Vector :type Vector))
  (return (/ Vector (Variables|Grid|GetCellSize))))

(fn WorldtoGrid
  (params (Input :type Vector))
  (bind _grid (Variables|Internal|GetGrid))
  (bind _returnvalue (Transformation|GetActorTransform _grid))
  (return (/ (Math|Vector|RotateVector (- Input (.location _returnvalue)) (Class|KismetMathLibrary|NegateRotator (.rotation _returnvalue))) (.scale _returnvalue))))